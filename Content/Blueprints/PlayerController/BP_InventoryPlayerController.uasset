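; Player controller that lets a client switch between three inventory save slots with the 1, 2 and 3 keys, marked as test functionality.
; Each key sets the slot name, loads that inventory save game locally and passes its contents to the inventory character through a server load call.
; The in-game widget then shows the active slot number.
; The key handlers do nothing when running on the server.
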(event `Key|One`
  (params (Key :type "Key Structure"))
  ;[1 1 1] Test function
  (:`Pressed`
    (if (not (`KismetSystemLibrary.IsServer`))
      (set `self.Inventory_SlotName` "InventorySlot_01")
      (`self.LoadInventorySaveGame`)
      (`InventoryCharacter.Server_LoadInventoryFromSaveGame` (`self.InventoryCharacter`) (`PlayerInventorySaveGame.GetPlayerInventory` (`self.PlayerInventorySaveGame`)))
      (`IngameWidget.Set_SaveSlotText` (`self.IngameWidget`) "1"))))

(event `Key|Two`
  (params (Key :type "Key Structure"))
  ;[1 1 1] Test function
  (:`Pressed`
    (if (not (`KismetSystemLibrary.IsServer`))
      (set `self.Inventory_SlotName` "InventorySlot_02")
      (`self.LoadInventorySaveGame`)
      (`InventoryCharacter.Server_LoadInventoryFromSaveGame` (`self.InventoryCharacter`) (`PlayerInventorySaveGame.GetPlayerInventory` (`self.PlayerInventorySaveGame`)))
      (`IngameWidget.Set_SaveSlotText` (`self.IngameWidget`) "2"))))

(event `Key|Three`
  (params (Key :type "Key Structure"))
  ;[1 1 1] Test function
  (:`Pressed`
    (if (not (`KismetSystemLibrary.IsServer`))
      (set `self.Inventory_SlotName` "InventorySlot_03")
      (`self.LoadInventorySaveGame`)
      (`InventoryCharacter.Server_LoadInventoryFromSaveGame` (`self.InventoryCharacter`) (`PlayerInventorySaveGame.GetPlayerInventory` (`self.PlayerInventorySaveGame`)))
      (`IngameWidget.Set_SaveSlotText` (`self.IngameWidget`) "3"))))

(fn `UserConstructionScript`)